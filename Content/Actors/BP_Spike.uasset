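; BP_Spike is a timed spike trap that damages the player character on overlap.
; On BeginPlay it drops the spikes below their placed position and starts a looping timer.
; Each cycle activates the Box, snaps the spikes up with MoveComponentTo, deactivates the Box, then retracts them more slowly after a delay.
; Box overlaps cast to AbstractionPlayerCharacter and apply heavy damage through TakeDamage.
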(event OnComponentBeginOverlap(Box)
  (params (OverlappedComponent :type Primitive%20Component%20Object%20Reference) (OtherActor :type Actor%20Object%20Reference) (OtherComp :type Primitive%20Component%20Object%20Reference) (OtherBodyIndex :type Integer) (bFromSweep :type Boolean) (SweepResult :type Hit%20Result%20Structure%20%28by%20ref%29))
  (bind _asabstraction_player_character (Utilities|Casting|CastToAbstractionPlayerCharacter OtherActor))
  (Class|AbstractionPlayerCharacter|TakeDamage _asabstraction_player_character 1e+02 (Utilities|Struct|MakeDamageEvent) 0 self))

(event Custom|ActivateTrap_Event
  (bind _spikes (Variables|Default|GetSpikes))
  (bind _spikebeginpos (Variables|Default|GetSpikeBeginPos))
  (bind _box (Variables|Default|GetBox))
  (Components|Activation|Activate _box false)
  (Components|MoveComponentTo _spikes _spikebeginpos "0, 0, 0" true true 0.1 false)
  (Components|Activation|Deactivate _box)
  (Utilities|FlowControl|Delay 1.0)
  (Components|MoveComponentTo _spikes (+ _spikebeginpos "0, 0,-100.000000") "0, 0, 0" true true 0.5 false))

(event EventBeginPlay
  (bind _spikes (Variables|Default|GetSpikes))
  (bind _relativelocation (Variables|/Script/Engine.SceneComponent|GetRelativeLocation _spikes))
  (Components|Activation|Deactivate (Variables|Default|GetBox))
  (Variables|Default|SetSpikeBeginPos _relativelocation)
  (Transformation|SetRelativeLocation _spikes (+ _relativelocation "0, 0,-100.000000") false true)
  (bind _returnvalue (Utilities|Time|SetTimerbyEvent (delegate Custom|ActivateTrap_Event) 5.0 true))
  (Variables|Default|SetTimerHandle _returnvalue))

(event Collision|EventActorBeginOverlap
  (params (OtherActor :type Actor%20Object%20Reference)))

(event EventTick
  (params (DeltaSeconds :type Float%20%28single-precision%29)))

(fn ConstructionScript)